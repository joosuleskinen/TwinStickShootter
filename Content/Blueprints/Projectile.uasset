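; Projectile Blueprint that deals damage to non-friendly actors it overlaps.
; On overlap, actors implementing IDamageable without the Friendly tag receive a health message with the Damage value and trigger an attached laser hit sound.
; Those hits and overlaps with non-damageable actors spawn laser sparks and destroy the projectile.
; Damageable actors tagged Friendly are ignored, leaving the projectile alive.
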(event EventBeginPlay)

(event Collision|EventActorBeginOverlap
  (params (OtherActor :type Actor%20Object%20Reference))
  (bind _returnvalue (Transformation|GetActorTransform))
  ;[1 1 1] Bullet affection
  (if (Utilities|DoesObjectImplementInterface OtherActor "/Game/Blueprints/IDamageable.IDamageable_C")
    (if (not (Actor|ActorHasTag OtherActor "Friendly")) ; If not friendly -> affect health
      (Class|IDamageable|AffectHealth(Message) OtherActor (Variables|Default|GetDamage))
      (Audio|SpawnSoundAttached "/Game/Audio/laser-hit.laser-hit" (Variables|Default|GetProjectileCollision) "None" "0, 0, 0" "0, 0, 0" "KeepRelativeOffset" false 1.0 1.0 0.0 0 0) ; Make hit sound when hit enemy
      (Effects|SpawnEmitteratLocation "/Game/StarterContent/Particles/LaserSparks.LaserSparks" (.location _returnvalue) (.rotation _returnvalue) :!label _label)
      (Actor|DestroyActor))
    (else
      (goto _label))))

(event EventTick
  (params (DeltaSeconds :type Float%20%28single-precision%29)))

(fn ConstructionScript)