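; Weapon actor Blueprint that fires automatic laser shots while the trigger is held.
; PullTrigger passes a DoOnce, fires immediately and starts a looping timer at the rounds-per-second rate; ReleaseTrigger clears the timer and resets the DoOnce.
; Each Fire checks that the player's HeroCharacter is alive, then plays an attached laser sound on the gun mesh and spawns a projectile at the spawn point.
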(event Custom|PullTrigger
  ;[1 1 1] When get input to fire call fire function
  (Utilities|FlowControl|DoOnce false
    (:Completed
      (CallFunction|Fire)
      (Utilities|Time|SetTimerbyFunctionName 0 "Fire" (/ 1.0 (Variables|Default|GetRoundsPerSecound)) true))))

(event Custom|ReleaseTrigger
  ;[1 1 1] When get input to fire call fire function
  (Utilities|Time|ClearTimerbyFunctionName 0 "Fire")
  (Utilities|FlowControl|DoOnce false) ; enters at Reset
)

(event Custom|Fire
  ;[1 1 1] Fire
  (bind _ashero_character (Utilities|Casting|CastToHeroCharacter (Game|GetPlayerCharacter 0)))
  (if (not (Variables|/Script/TwinStickShootter.BaseCharacter|GetisDead _ashero_character))
    (Audio|SpawnSoundAttached "/Game/Audio/laser-shot.laser-shot" (Variables|Default|GetGunMesh) "None" "0, 0, 0" "0, 0, 0" "KeepRelativeOffset" false 1.0 1.0 0.0 0 0)
    (Game|SpawnActorfromClass "/Game/Blueprints/Projectile.Projectile_C" (Transformation|GetWorldTransform (Variables|Default|GetProjectileSpawnPoint)) "Undefined" "MultiplyWithRoot" 0 0)))

(event EventBeginPlay)

(event Collision|EventActorBeginOverlap
  (params (OtherActor :type Actor%20Object%20Reference)))

(event EventTick
  (params (DeltaSeconds :type Float%20%28single-precision%29)))

(fn ConstructionScript)