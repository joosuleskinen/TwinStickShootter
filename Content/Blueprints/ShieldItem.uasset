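; Shield pickup item that gives an overlapping HeroCharacter a shield when their shield HP is below full.
; A successful pickup calls AttachShield, plays a sound, decrements the ItemSpawner's shield count and destroys the item; otherwise a rejection sound plays.
; If the Shield component overlaps a component whose last-iterated tag is ItemSpawnBlocker, the item moves to a random spot within the spawner's volume at fixed height.
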(event OnComponentBeginOverlap(Shield)
  (params (OverlappedComponent :type Primitive%20Component%20Object%20Reference) (OtherActor :type Actor%20Object%20Reference) (OtherComp :type Primitive%20Component%20Object%20Reference) (OtherBodyIndex :type Integer) (bFromSweep :type Boolean) (SweepResult :type Hit%20Result%20Structure%20%28by%20ref%29))
  ;[1 1 1] If shield inside walls move it
  (for _array_element (Variables|/Script/Engine.ActorComponent|GetComponentTags OtherComp)
    _)
  (if (== _array_element "ItemSpawnBlocker")
    (bind _returnvalue (Actor|GetActorOfClass "/Game/Blueprints/ItemSpawner.ItemSpawner_C"))
    (Transformation|SetActorLocation (Math|Vector|MakeVector (.x (Math|Random|RandomPointinBoundingBox (Transformation|GetWorldLocation (Variables|/Game/Blueprints/ItemSpawner.ItemSpawner_C|GetSpawnVolume _returnvalue)) (Components|Box|GetScaledBoxExtent (Variables|/Game/Blueprints/ItemSpawner.ItemSpawner_C|GetSpawnVolume _returnvalue)))) (.y (Math|Random|RandomPointinBoundingBox (Transformation|GetWorldLocation (Variables|/Game/Blueprints/ItemSpawner.ItemSpawner_C|GetSpawnVolume _returnvalue)) (Components|Box|GetScaledBoxExtent (Variables|/Game/Blueprints/ItemSpawner.ItemSpawner_C|GetSpawnVolume _returnvalue)))) 125.0) false false) ; Shield new location
  ))

(event EventBeginPlay)

(event Collision|EventActorBeginOverlap
  (params (OtherActor :type Actor%20Object%20Reference))
  ;[1 1 1] When player pick shield item
  (bind _ashero_character (Utilities|Casting|CastToHeroCharacter OtherActor))
  (if (> 6e+01 (Variables|/Game/Blueprints/HeroCharacter.HeroCharacter_C|GetShieldHP _ashero_character)) ; If shield have full helth dont pick it
    (Default|AttachShield _ashero_character)
    (Audio|SpawnSoundAttached "/Game/Audio/item-pickup-sound.item-pickup-sound" (Variables|/Script/Engine.Character|GetMesh _ashero_character) "None" "0, 0, 0" "0, 0, 0" "KeepRelativeOffset" false 1.0 1.0 0.0 0 0) ; pick up sound
    ;;[1 1 1] Item counter - 1 when picked shield
    (bind _returnvalue (Actor|GetActorOfClass "/Game/Blueprints/ItemSpawner.ItemSpawner_C"))
    (bind _asitem_spawner (Utilities|Casting|CastToItemSpawner _returnvalue))
    (Variables|/Game/Blueprints/ItemSpawner.ItemSpawner_C|SetShieldItemCount _asitem_spawner (- (Variables|/Game/Blueprints/ItemSpawner.ItemSpawner_C|GetShieldItemCount _asitem_spawner) 1))
    (Actor|DestroyActor)
    (else
      (Audio|SpawnSoundAttached "/Game/Audio/item-not-pickup-sound.item-not-pickup-sound" (Variables|/Script/Engine.Character|GetMesh _ashero_character) "None" "0, 0, 0" "0, 0, 0" "KeepRelativeOffset" false 1.0 1.0 0.0 0 0) ; Cannot pick up sound
    )))

(event EventTick
  (params (DeltaSeconds :type Float%20%28single-precision%29)))

(fn ConstructionScript)