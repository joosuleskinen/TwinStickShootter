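; EnemyCharacter is a twin-stick shooter enemy that damages the hero while overlapping it and awards score when killed.
; BeginPlay boosts walk speed by TwinStickMode's difficulty increment, and the construction script tints the body through a dynamic material.
; Overlap starts a looping damage timer at AttacksPerSecond.
; On death it drops pawn collision, detaches its controller, reports score to TwinStickMode, then explodes and destroys itself after a delay.
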(event Custom|DamageTheHero
  ;[1 1 1] Reduce heroes (player) health
  (bind _ashero_character (Utilities|Casting|CastToHeroCharacter (Variables|Default|GetHero)))
  (if (not (Variables|/Script/TwinStickShootter.BaseCharacter|GetisDead _ashero_character))
    (Default|AffectHealth (Variables|Default|GetHero) (Variables|Default|GetDamage))))

(event EventBeginPlay
  (bind _charactermovement (Variables|Character|GetCharacterMovement))
  ;[1 1 1] Increas max walk speed
  (bind _returnvalue (Actor|GetActorOfClass "/Game/Blueprints/TwinStickMode.TwinStickMode_C"))
  (bind _astwin_stick_mode (Utilities|Casting|CastToTwinStickMode _returnvalue))
  (Variables|/Script/Engine.CharacterMovementComponent|SetMaxWalkSpeed _charactermovement (+ (Variables|/Script/Engine.CharacterMovementComponent|GetMaxWalkSpeed _charactermovement) (Variables|/Game/Blueprints/TwinStickMode.TwinStickMode_C|GetEnemiesSpeedIncrement _astwin_stick_mode))))

(event Collision|EventActorBeginOverlap
  (params (OtherActor :type Actor%20Object%20Reference))
  ;[1 1 1] Make damage to hero (player)
  (bind _ashero_character (Utilities|Casting|CastToHeroCharacter OtherActor))
  (Variables|Default|SetHero _ashero_character)
  (Utilities|Time|SetTimerbyFunctionName 0 "DamageTheHero" (/ 1.0 (Variables|Default|GetAttacksPerSecond)) true))

(event EventTick
  (params (DeltaSeconds :type Float%20%28single-precision%29)))

(event EventAffectHealth
  (params (Delta :type Float%20%28double-precision%29))
  (bind _capsulecomponent (Variables|Default|GetCapsuleComponent))
  ;[1 1 1] Destroy enemy when no health
  (Class|BaseCharacter|CalculateHealth Delta)
  (if (Variables|Default|GetisDead)
    (Collision|SetCollisionResponsetoChannel _capsulecomponent "ECC_WorldDynamic" "ECR_Ignore") ; can go trought dead bodies
    (Collision|SetCollisionResponsetoChannel _capsulecomponent "ECC_Pawn" "ECR_Ignore") ; can go trought dead bodies
    (Class|Pawn|DetachfromControllerPendingDestroy)
    (bind _astwin_stick_mode (Utilities|Casting|CastToTwinStickMode (Game|GetGameMode)))
    (Default|IncrementScore _astwin_stick_mode (Variables|Default|GetScore)) ; Add score when enemy is destroyed
    ;;[1 1 1] Count scores and change difficult every +5000 score
    (bind _returnvalue (Actor|GetActorOfClass "/Game/Blueprints/TwinStickMode.TwinStickMode_C"))
    (bind _astwin_stick_mode_2 (Utilities|Casting|CastToTwinStickMode _returnvalue))
    (Default|CalculateScore _astwin_stick_mode_2 (Variables|Default|GetScore))
    (Utilities|FlowControl|Delay 3.0)
    (Game|SpawnActorfromClass "/Game/Blueprints/Explosion.Explosion_C" (Transformation|GetActorTransform) "Undefined" "MultiplyWithRoot" 0 0) ; Explosion effect
    (Actor|DestroyActor)))

(event Collision|EventActorEndOverlap
  (params (OtherActor :type Actor%20Object%20Reference))
  ;[1 1 1] End damage to hero (player)
  (if (== OtherActor (Variables|Default|GetHero))
    (Utilities|Time|ClearTimerbyFunctionName 0 "DamageTheHero")))

(fn ConstructionScript
  ;[1 1 1] Add enemey color
  (bind _returnvalue (Rendering|Material|CreateDynamicMaterialInstance (Variables|Character|GetMesh) 0 0 "None" :!class /Script/Engine.PrimitiveComponent))
  (bind _output_get (Variables|Default|SetDynaMat _returnvalue))
  (Rendering|Material|SetVectorParameterValue _output_get "BodyColor" (Variables|Default|GetEnemyColor) :!class /Script/Engine.MaterialInstanceDynamic))